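; BP_Barrel is an explosive barrel actor that blows up when hit or damaged.
; Both triggers call Explode, which a flag limits to one run and which waits a configurable delay.
; It then spawns an actor, plays a sound, fires a radial force impulse and applies radial damage over the same radius before destroying itself.
; Since any damage triggers Explode, the blast can chain to neighboring barrels.
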(event `self.ReceiveHit`
  (params (MyComp :type "PrimitiveComponent Object Reference") (Other :type "Actor Object Reference") (OtherComp :type "PrimitiveComponent Object Reference") (bSelfMoved :type Boolean) (HitLocation :type "Vector Structure") (HitNormal :type "Vector Structure") (NormalImpulse :type "Vector Structure") (Hit :type "HitResult Structure (by ref)"))
  (`self.Explode` :!label _label))

(event `self.ReceiveAnyDamage`
  (params (Damage :type "Float (single-precision)") (DamageType :type "DamageType Object Reference") (InstigatedBy :type "Controller Object Reference") (DamageCauser :type "Actor Object Reference"))
  (goto _label))

(event `Explode`
  (bind _radialforce (`self.RadialForce`))
  (bind _returnvalue (`SceneComponent.K2_GetComponentLocation` (`self.Barrel`)))
  ; Explosion flow
  (if (not (`self.isExploded`))
    (set `self.isExploded` true)
    (`KismetSystemLibrary.Delay` (`self.waitOffset`))
    (`|SpawnActorFromClass` "/Game/Variant_Shooter/Blueprints/Pickups/Projectiles/BP_Shooter_GrenadeExplosion.BP_Shooter_GrenadeExplosion_C" (`KismetMathLibrary.MakeTransform` _returnvalue) "Undefined" "MultiplyWithRoot" null null)
    (`GameplayStatics.PlaySoundAtLocation` "/Game/Weapons/GrenadeLauncher/Audio/FirstPersonTemplateWeaponFire02.FirstPersonTemplateWeaponFire02" _returnvalue (struct) 1.0 1.0 0.0 null null null null)
    (set `RadialForceComponent.Radius` (`self.Radius`) _radialforce) ; In Radial Force there is Radial Force Component that uses Radius
    (`RadialForceComponent.FireImpulse` _radialforce)
    (`GameplayStatics.ApplyRadialDamage` (`self.Damage`) _returnvalue (`self.Radius`) null (`|MakeArray` self :!type "Actor Object Reference") null null)
    (`self.K2_DestroyActor`)))

(fn `UserConstructionScript`)